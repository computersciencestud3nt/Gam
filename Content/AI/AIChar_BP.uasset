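; AI bot character for a shooter that fires AIProj_BP projectiles at any pawn it sees.
; PawnSensing turns the bot toward the target and shoots on a short cooldown; the timer-driven AIShoot event is empty.
; Damage updates an overhead health widget that yaws toward the player.
; At zero health it drops far below the map, then respawns at a random AI_Spawn with health reset to 100.
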(event OnSeePawn(PawnSensing)
  (params (Pawn :type Pawn%20Object%20Reference))
  ;[0.15 0.15 0.15 0.5] look at character
  (Transformation|SetActorRotation (Math|Rotator|FindRelativeLookatRotation (Math|Conversions|ToTransform(Vector) (Transformation|GetActorLocation)) (Transformation|GetActorLocation Pawn)))
  ;[0.15 0.15 0.15 0.5] Created Proyectile
  (if (Variables|Default|GetCanAttack?)
    (Game|SpawnActorfromClass "/Game/AI/AIProj_BP.AIProj_BP_C" (Transformation|GetWorldTransform (Variables|Default|GetArrow1)) "Undefined" "MultiplyWithRoot" 0 0)
    ;[0.15 0.15 0.15 0.5] Delays Attack
    (Variables|Default|SetCanAttack? false)
    (Utilities|FlowControl|Delay 0.8)
    (Variables|Default|SetCanAttack? true)))

(event Custom|Respawn
  (bind _aispawn (Variables|Default|GetAISPawn))
  ;[0.15 0.15 0.15 0.5] Respawn
  (Utilities|FlowControl|Delay 0.2)
  (Variables|Default|SetHealth 1e+02)
  (Transformation|SetActorLocation (Transformation|GetActorLocation (Utilities|Array|Get(acopy) _aispawn (Math|Random|RandomIntegerinRange 0 (- (Utilities|Array|Length _aispawn) 1)))) false false)
  (Default|SetHealth (Variables|Default|GetAs%20AI%20W) (Variables|Default|GetHealth) (Variables|Default|GetMaxHealth)))

(event Custom|StartShooting
  (Utilities|Time|SetTimerbyFunctionName 0 "AIShoot" (Variables|Default|GetRateofFire) true))

(event Custom|AddScore
  (params (Value :type Integer))
  ;[0.15 0.15 0.15 0.5] Add score
  (Variables|Default|SetScore (+ (Variables|Default|GetScore) Value)))

(event Custom|StopShooting
  (Utilities|Time|ClearTimerbyFunctionName 0 "AIShoot"))

(event Custom|CheckHealth
  (bind _damage_causer (Variables|Default|GetDamage%20Causer))
  ;[0.15 0.15 0.15 0.5] Check Health
  (if (<= (Variables|Default|GetHealth) 0.0)
    (bind _asaichar_bp (Utilities|Casting|CastToAIChar_BP _damage_causer))
    (CallFunction|AddScore _asaichar_bp 1)
    (else
      (bind _asplayer_char_bp (Utilities|Casting|CastToPlayerChar_BP _damage_causer))
      (Default|AddScore _asplayer_char_bp 1))))

(event Custom|AIShoot
  ;[0.15 0.15 0.15 0.5] Creates projectile
)

(event EventTick
  (params (DeltaSeconds :type Float%20%28single-precision%29))
  (bind _widget (Variables|Default|GetWidget))
  ;[0.15 0.15 0.15 0.5] Life bar is looking at player
  (Transformation|SetWorldRotation _widget (Math|Rotator|MakeRotator 0.0 0.0 (.yaw (Math|Rotator|FindLookatRotation (Transformation|GetWorldLocation _widget) (Transformation|GetActorLocation (Game|GetPlayerCharacter 0))))) false false))

(event EventBeginPlay
  ;[0.15 0.15 0.15 0.5] ADD Name to Scoreboard ANd load SPawn points
  (bind _outactors (Actor|GetAllActorsOfClass "/Game/Spawn/AI_Spawn.AI_Spawn_C"))
  (Variables|Default|SetAISPawn _outactors)
  (Variables|Default|SetName (Utilities|Text|ToText(String) (Utilities|String|Append "Bot#:" (Utilities|String|ToString(Integer) (Math|Random|RandomInteger 500)))))
  (bind _asai_w (Utilities|Casting|CastToAI_W (UserInterface|GetUserWidgetObject (Variables|Default|GetWidget))))
  (Variables|Default|SetAs%20AI%20W _asai_w))

(event Game|Damage|EventAnyDamage
  (params (Damage :type Float%20%28single-precision%29) (DamageType :type Damage%20Type%20Object%20Reference) (InstigatedBy :type Controller%20Object%20Reference) (DamageCauser :type Actor%20Object%20Reference))
  ;[0.15 0.15 0.15 0.5] Print health
  (bind _output_get (Variables|Default|SetHealth (- (Variables|Default|GetHealth) Damage)))
  (Development|PrintString (Utilities|String|ToString(Float) _output_get) true true "(R=0.003933,G=1.000000,B=0.004833,A=1.000000)")
  ;[0.15 0.15 0.15 0.5] Damage to ai and if at 0 Respawn
  (Default|SetHealth (Variables|Default|GetAs%20AI%20W) (Variables|Default|GetHealth) (Variables|Default|GetMaxHealth))
  (if (<= (Variables|Default|GetHealth) 0.0)
    (Transformation|SetActorLocation "0.000000,0.000000,-50000.000000" false false)
    (CallFunction|Respawn)))

(fn ConstructionScript)